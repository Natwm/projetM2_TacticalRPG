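; Basic spell for a grid-based tactics game that highlights targetable tiles and damages an opposing unit.
; Showing targets clears the previous highlight, then asks GetReachableTarget for tiles within the spell's distance and highlights them through the Grid.
; GetReachableTarget scans grid tiles by occupant, type and estimated cost, then returns the result of the Grid's pathfinder in reachable mode.
; Casting damages the tile's character unless it shares the caster's owner or stands on two excluded tile types.
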(event `E_ShowTilesTargetedBySpell`
  (params (`Origin Index` :type "Vector2D Structure") (Grid :type "/Game/01_BP/Grid/GridBehaviours Object Reference"))
  (if (> (`KismetArrayLibrary.Array_Length` (`self.ReachableTarger`)) 0)
    (`/Game/01_BP/Grid/GridBehaviours.Highlight Attackable Tiles` Grid (`self.ReachableTarger`) false)
    (`KismetArrayLibrary.Array_Clear` (`self.ReachableTarger`)))
  (bind _reachable_tiles (`self.GetReachableTarget` `Origin Index` (`self.m_Distances`) Grid))
  (bind _output_get (set `self.ReachableTarger` _reachable_tiles))
  (`/Game/01_BP/Grid/GridBehaviours.Highlight Attackable Tiles` Grid _output_get true))

(event `E_UseSpellOnTarget`
  (params (Grid :type "/Game/01_BP/Grid/GridBehaviours Object Reference") (`Target position` :type "Vector2D Structure") (SpellOwner :type "/Game/01_BP/03_Character/TopDownCharacter Object Reference"))
  (bind _value (`BlueprintMapLibrary.Map_Find` (`/Game/01_BP/Grid/GridBehaviours.struct_Tiles` Grid) `Target position`))
  (bind (_astop_down_character _bsuccess) (cast `/Game/01_BP/03_Character/TopDownCharacter` (`.UnitOnThisTile_34_604DD03C40109D7673B4448C065FC6E9` (break `/Game/01_BP/Structure/Tiles_Struct` _value)) :!pure true))
  (if (and _bsuccess (`|EnumInequality` (`.m_TypesOfTile_9_31305E934CC54E66306D4C98AE8F7317` (break `/Game/01_BP/Structure/Tiles_Struct` _value)) "NewEnumerator5") (`|EnumInequality` (`.m_TypesOfTile_9_31305E934CC54E66306D4C98AE8F7317` (break `/Game/01_BP/Structure/Tiles_Struct` _value)) "NewEnumerator6") (`|EnumInequality` (`/Game/01_BP/03_Character/TopDownCharacter.m_PawnOwner` _astop_down_character) (`/Game/01_BP/03_Character/TopDownCharacter.m_PawnOwner` SpellOwner)))
    (`/Game/01_BP/03_Character/TopDownCharacter.E_TakeDamage` _astop_down_character (`self.m_Degats`))))

(fn `GetReachableTarget`
  (params (`Origin Index` :type "Vector2D Structure") (Distance :type Integer) (Grid :type "/Game/01_BP/Grid/GridBehaviours Object Reference"))
  (returns (`Reachable Tiles` :type "Array of Vector2D Structure"))
  (locals (FirstIndex :type "Vector2D Structure") (m_Distance :type Integer) (TargetIndex :type "Vector2D Structure"))
  (set `local.FirstIndex` `Origin Index`)
  (set `local.m_Distance` Distance)
  (bind _keys (`BlueprintMapLibrary.Map_Keys` (`/Game/01_BP/Grid/GridBehaviours.struct_Tiles` Grid)))
  (for _array_element _keys
    (bind _output_get (set `local.TargetIndex` _array_element))
    (bind _value (`BlueprintMapLibrary.Map_Find` (`/Game/01_BP/Grid/GridBehaviours.struct_Tiles` Grid) _output_get))
    (if (or (!= (`.UnitOnThisTile_34_604DD03C40109D7673B4448C065FC6E9` (break `/Game/01_BP/Structure/Tiles_Struct` _value)) null) (`|EnumEquality` (`.m_TypesOfTile_9_31305E934CC54E66306D4C98AE8F7317` (break `/Game/01_BP/Structure/Tiles_Struct` _value)) "NewEnumerator6") (`|EnumEquality` (`.m_TypesOfTile_9_31305E934CC54E66306D4C98AE8F7317` (break `/Game/01_BP/Structure/Tiles_Struct` _value)) "NewEnumerator5") (> (`/Game/01_BP/Grid/GridBehaviours.Get EstimatedCostToTarget` Grid (`local.FirstIndex`) (`local.TargetIndex`)) (`local.m_Distance`)))
      (break)))
  (bind _reachable_tiles (`/Game/01_BP/Grid/GridBehaviours.FindPathToTarget` Grid (`local.FirstIndex`) (`local.TargetIndex`) (`local.m_Distance`) true))
  (return _reachable_tiles))

(fn `test`)

(fn `UserConstructionScript`)