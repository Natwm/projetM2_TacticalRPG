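; Tank spell that damages an enemy character on a grid tile, excluding two tile types, and knocks it away from the caster.
; PushActionResult finds the landing tile by adding the caster-to-target index offset to the target's index, then moves the target there if unoccupied.
; If blocked, a character there takes half damage, while an obstacle gives the pushed target a speed debuff.
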(event `self.E_UseSpellOnTarget`
  (params (Grid :type "/Game/01_BP/Grid/GridBehaviours Object Reference") (`Target position` :type "Vector2D Structure") (SpellOwner :type "/Game/01_BP/03_Character/TopDownCharacter Object Reference"))
  (bind _value (`BlueprintMapLibrary.Map_Find` (`/Game/01_BP/Grid/GridBehaviours.struct_Tiles` Grid) `Target position`))
  (bind (_astop_down_character _bsuccess) (cast `/Game/01_BP/03_Character/TopDownCharacter` (`.UnitOnThisTile_34_604DD03C40109D7673B4448C065FC6E9` (break `/Game/01_BP/Structure/Tiles_Struct` _value)) :!pure true))
  (if (and _bsuccess (`|EnumInequality` (`.m_TypesOfTile_9_31305E934CC54E66306D4C98AE8F7317` (break `/Game/01_BP/Structure/Tiles_Struct` _value)) "NewEnumerator5") (`|EnumInequality` (`.m_TypesOfTile_9_31305E934CC54E66306D4C98AE8F7317` (break `/Game/01_BP/Structure/Tiles_Struct` _value)) "NewEnumerator6") (`|EnumInequality` (`/Game/01_BP/03_Character/TopDownCharacter.m_PawnOwner` _astop_down_character) (`/Game/01_BP/03_Character/TopDownCharacter.m_PawnOwner` SpellOwner)))
    (`/Game/01_BP/03_Character/TopDownCharacter.E_TakeDamage` _astop_down_character (`self.m_Degats`))
    (`self.PushActionResult` _astop_down_character SpellOwner Grid)
    (set `/Game/01_BP/03_Character/TopDownCharacter.CurrentSpell` null SpellOwner)))

(fn `PushActionResult`
  (params (SpeelTarget :type "/Game/01_BP/03_Character/TopDownCharacter Object Reference") (SpeelCaster :type "/Game/01_BP/03_Character/TopDownCharacter Object Reference") (GridManager :type "/Game/01_BP/Grid/GridBehaviours Object Reference"))
  (locals (Target :type "/Game/01_BP/03_Character/TopDownCharacter Object Reference") (Caster :type "/Game/01_BP/03_Character/TopDownCharacter Object Reference") (Grid :type "/Game/01_BP/Grid/GridBehaviours Object Reference"))
  (bind _grid_index (`/Game/01_BP/03_Character/TopDownCharacter.grid Index` (`local.Target`)))
  (bind _value (`BlueprintMapLibrary.Map_Find` (`/Game/01_BP/Grid/GridBehaviours.struct_Tiles` (`local.Grid`)) (+ _grid_index (- _grid_index (`/Game/01_BP/03_Character/TopDownCharacter.grid Index` (`local.Caster`))))))
  (bind (_astop_down_character _bsuccess) (cast `/Game/01_BP/03_Character/TopDownCharacter` (`.UnitOnThisTile_34_604DD03C40109D7673B4448C065FC6E9` (break `/Game/01_BP/Structure/Tiles_Struct` _value)) :!pure true))
  (set `local.Target` SpeelTarget)
  (set `local.Caster` SpeelCaster)
  (set `local.Grid` GridManager)
  (if (== (`.UnitOnThisTile_34_604DD03C40109D7673B4448C065FC6E9` (break `/Game/01_BP/Structure/Tiles_Struct` _value)) null)
    (`self.K2_SetActorLocation` (`local.Target`) (`.m_Tiles_WorldLocation_10_52D11E814B5D8A10CE64A1B92294C51C` (break `/Game/01_BP/Structure/Tiles_Struct` _value)) false false)
    (set `/Game/01_BP/03_Character/TopDownCharacter.grid Index` (`.m_Tiles_Index_12_B076B1C84440D5EFB37DCB994C2C5E0D` (break `/Game/01_BP/Structure/Tiles_Struct` _value)) (`local.Target`))
    (elif _bsuccess
      (`/Game/01_BP/03_Character/TopDownCharacter.E_TakeDamage` _astop_down_character (/ (`self.m_Degats`) 2))
      (else
        ;[1 1 1] Apply a debuf on the speed
        (if (`.bSuccess` (cast `/Game/01_BP/Obstacles/BP_Base_Obstacle` (`.UnitOnThisTile_34_604DD03C40109D7673B4448C065FC6E9` (break `/Game/01_BP/Structure/Tiles_Struct` _value)) :!pure true))
          (`/Game/01_BP/03_Character/TopDownCharacter.E_ApplyDebuff` (`local.Target`) 1))))))

(fn `UserConstructionScript`
  (`parent.UserConstructionScript`))