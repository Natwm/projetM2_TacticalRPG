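; BP_Bond is a Rushdown spell that leaps its caster to a target tile on the tactical grid.
; It looks up the tile in StructTiles and checks for no occupying TopDownCharacter, two excluded tile types and an owner mismatch.
; On success it moves the caster to the tile's world location and updates its GridIndex, without updating tile occupancy.
; A noted height-based area damage effect is an unconnected stub.
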(event `self.E_UseSpellOnTarget`
  (params (Grid :type "/Game/01_BP/Grid/GridBehaviours Object Reference") (`Target position` :type "Vector2D Structure") (SpellOwner :type "/Game/01_BP/03_Character/TopDownCharacter Object Reference"))
  (bind _spellowner (`self.SpellOwner`))
  (bind _value (`BlueprintMapLibrary.Map_Find` (`/Game/01_BP/Grid/GridBehaviours.struct_Tiles` Grid) `Target position`))
  (bind (_astop_down_character _bsuccess) (cast `/Game/01_BP/03_Character/TopDownCharacter` (`.UnitOnThisTile_34_604DD03C40109D7673B4448C065FC6E9` (break `/Game/01_BP/Structure/Tiles_Struct` _value)) :!pure true))
  (if (and (not _bsuccess) (`|EnumInequality` (`.m_TypesOfTile_9_31305E934CC54E66306D4C98AE8F7317` (break `/Game/01_BP/Structure/Tiles_Struct` _value)) "NewEnumerator5") (`|EnumInequality` (`.m_TypesOfTile_9_31305E934CC54E66306D4C98AE8F7317` (break `/Game/01_BP/Structure/Tiles_Struct` _value)) "NewEnumerator6") (`|EnumInequality` (`/Game/01_BP/03_Character/TopDownCharacter.m_PawnOwner` _astop_down_character) (`/Game/01_BP/03_Character/TopDownCharacter.m_PawnOwner` SpellOwner)))
    (`self.K2_SetActorLocation` _spellowner (`.m_Tiles_WorldLocation_10_52D11E814B5D8A10CE64A1B92294C51C` (break `/Game/01_BP/Structure/Tiles_Struct` _value)) false false)
    (set `/Game/01_BP/03_Character/TopDownCharacter.grid Index` (`.m_Tiles_Index_12_B076B1C84440D5EFB37DCB994C2C5E0D` (break `/Game/01_BP/Structure/Tiles_Struct` _value)) _spellowner)))

(fn `UserConstructionScript`
  (`parent.UserConstructionScript`))