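; BP_Rush is the Rushdown spell Blueprint, which computes the grid tiles affected by a straight-line rush.
; RushActionResult takes the SpellOwner-to-Target grid offset, using X if nonzero, otherwise Y.
; It adds unique tiles stepping in the positive axis direction from the owner, one fewer than that offset, to AffectedTiles and returns it.
; Only a positive owner-minus-target offset adds tiles, and they extend away from the target.
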(fn `RushActionResult`
  (params (target :type "Vector2D Structure"))
  (returns (AffectedTile :type "Array of Vector2D Structure"))
  (locals (AffectedTiles :type "Array of Vector2D Structure"))
  (bind (_x _y) (`KismetMathLibrary.BreakVector2D` (- (`/Game/01_BP/03_Character/TopDownCharacter.grid Index` (`self.SpellOwner`)) target)))
  (if (!= _x 0.0)
    (for _index (range 1 (`KismetMathLibrary.FTrunc` _x))
      (`KismetArrayLibrary.Array_AddUnique` (`local.AffectedTiles`) (+ (`/Game/01_BP/03_Character/TopDownCharacter.grid Index` (`self.SpellOwner`)) (`KismetMathLibrary.MakeVector2D` (`KismetMathLibrary.Conv_IntToDouble` _index)))))
    (return (`local.AffectedTiles`))
    (elif (!= _y 0.0)
      (for _index_2 (range 1 (`KismetMathLibrary.FTrunc` _y))
        (`KismetArrayLibrary.Array_AddUnique` (`local.AffectedTiles`) (+ (`/Game/01_BP/03_Character/TopDownCharacter.grid Index` (`self.SpellOwner`)) (`KismetMathLibrary.MakeVector2D` 0.0 (`KismetMathLibrary.Conv_IntToDouble` _index_2)))))
      (return (`local.AffectedTiles`)))))

(fn `UserConstructionScript`
  (`parent.UserConstructionScript`))