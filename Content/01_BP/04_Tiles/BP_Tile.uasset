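; BP_Tile is one clickable cell of the tile grid, showing its terrain type and current state through color.
; After a short delay on BeginPlay, it colors and flattens itself to the grid's tile size and passes grid and index to its W_GridTile widget.
; Mouse hover and clicks update its state and notify BPGrid.
; SetTilesColor layers reachable, attackable and path colors over the terrain color, brightens on hover, then sets a material parameter.
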(event `self.ReceiveBeginPlay`
  (bind _asw_grid_tile (cast `/Game/01_BP/Grid/W_GridTile` (`WidgetComponent.GetUserWidgetObject` (`self.Widget`)) :!pure true))
  (`KismetSystemLibrary.Delay` 0.2)
  (`self.SetTilesColor`)
  (`self.SetTilesSize`)
  (set `/Game/01_BP/Grid/W_GridTile.Grid` (`self.BP_Grid`) _asw_grid_tile)
  (set `/Game/01_BP/Grid/W_GridTile.GridIndex` (`self.Grid_Index`) _asw_grid_tile))

(event `self.StaticMesh.OnBeginCursorOver`
  (params (TouchedComponent :type "PrimitiveComponent Object Reference"))
  ;[1 1 1] Hover
  (`self.E_StartOverTile`)
  (`/Game/01_BP/Grid/GridBehaviours.E_NewTileOvered` (`self.BP_Grid`) self))

(event `self.StaticMesh.OnEndCursorOver`
  (params (TouchedComponent :type "PrimitiveComponent Object Reference"))
  ;[1 1 1] Hover
  (`/Game/01_BP/Grid/GridBehaviours.E_NewTileOvered` (`self.BP_Grid`) null))

(event `self.StaticMesh.OnClicked`
  (params (TouchedComponent :type "PrimitiveComponent Object Reference") (ButtonPressed :type "Key Structure"))
  ;[1 1 1] Selection Tiles
  (`self.E_SelectTiles`)
  (`/Game/01_BP/Grid/GridBehaviours.E_NewTilesSelected` (`self.BP_Grid`) self))

(event `E_SelectTiles`
  ;[1 1 1] Selection Deselection
  (set `self.IsSelected` true)
  (`self.SetTilesColor` :!label _label))

(event `E_DeselectTiles`
  ;[1 1 1] Selection Deselection
  (set `self.IsSelected` false)
  (goto _label))

(event `E_StartOverTile`
  ;[1 1 1] Over Tiles
  (set `self.IsOver` true)
  (`self.SetTilesColor` :!label _label_2))

(event `E_EndOverTiles`
  ;[1 1 1] Over Tiles
  (set `self.IsOver` false)
  (goto _label_2))

(event `E_IsInPath`
  (params (IsInPath :type Boolean))
  (set `self.Is in Path` IsInPath)
  (`self.SetTilesColor`))

(event `E_isReachable`
  (params (IsReachable :type Boolean))
  (set `self.IsReachable` IsReachable)
  (`self.SetTilesColor`))

(event `E_isAttackable`
  (params (IsAttackable :type Boolean))
  (set `self.IsAttackable` IsAttackable)
  (`self.SetTilesColor`))

(fn `GetTilesData`
  (returns (Data :type "/Game/01_BP/Structure/Tiles_Struct Structure"))
  (return (`BlueprintMapLibrary.Map_Find` (`/Game/01_BP/Grid/GridBehaviours.struct_Tiles` (`self.BP_Grid`)) (`self.Grid_Index`))))

(fn `SetTilesColor`
  (locals (TilesColor :type "LinearColor Structure"))
  (bind (_data_tileactor _data_unitonthistile _data_tilecost _data_m_typesoftile) (break `/Game/01_BP/Structure/Tiles_Struct` (`self.GetTilesData`)))
  (`|ExecutionSequence`
    (:`then_0`
      ;[1 1 1] Get Color
      (switch `/Game/01_BP/Enum/TileProfiles` _data_m_typesoftile
        (:`NewEnumerator0`
          (set `local.TilesColor` (struct :`R` 1.0 :`G` 0.96461 :`B` 0.60403 :`A` 1.0)))
        (:`NewEnumerator1`
          (set `local.TilesColor` (struct :`G` 1.0 :`A` 1.0)))
        (:`NewEnumerator2`
          (set `local.TilesColor` (struct :`B` 1.0 :`A` 1.0)))
        (:`NewEnumerator3`
          (set `local.TilesColor` (struct :`R` 1.0 :`G` 1.0 :`A` 1.0)))
        (:`NewEnumerator4`
          (set `local.TilesColor` (struct :`R` 1.0 :`B` 1.0 :`A` 1.0)))
        (:`NewEnumerator5`
          (set `local.TilesColor` (struct :`R` 1.0 :`A` 1.0)))
        (:`NewEnumerator6`
          (set `local.TilesColor` (struct :`A` 1.0)))))
    (:`then_1`
      (if (`self.IsReachable`)
        (set `local.TilesColor` (struct :`R` 0.565861 :`G` 0.781075 :`B` 1.0 :`A` 1.0))))
    (:`then_2`
      (if (`self.IsAttackable`)
        (set `local.TilesColor` (struct :`R` 1.0 :`G` 0.186303 :`B` 0.166406 :`A` 1.0))))
    (:`then_3`
      (if (`self.Is in Path`)
        (set `local.TilesColor` (struct :`R` 1.0 :`G` 1.0 :`B` 1.0 :`A` 1.0))))
    (:`then_4`
      (if (`self.IsOver`)
        (set `local.TilesColor` (`KismetMathLibrary.Conv_VectorToLinearColor` (* (`KismetMathLibrary.Conv_LinearColorToVector` (`local.TilesColor`)) 3.0)))))
    (:`then_5`
      ;[1 1 1] Set Color
      (`MeshComponent.SetVectorParameterValueOnMaterials` (`self.StaticMesh`) "ColorParam" (`KismetMathLibrary.Conv_LinearColorToVector` (`local.TilesColor`))))))

(fn `SetTilesSize`
  (bind (_returnvalue_x _returnvalue_y) (`KismetMathLibrary.BreakVector` (* (`SceneComponent.K2_GetComponentScale` (`self.StaticMesh`)) (/ (`/Game/01_BP/Grid/GridBehaviours.Tiles Size` (`self.BP_Grid`)) 50.0))))
  (`SceneComponent.SetWorldScale3D` (`self.StaticMesh`) (`KismetMathLibrary.MakeVector` _returnvalue_x _returnvalue_y)))

(fn `UserConstructionScript`)