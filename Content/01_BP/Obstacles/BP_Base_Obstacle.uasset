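; Base obstacle actor that snaps itself onto the tile grid and registers as that tile's occupant.
; Shortly after BeginPlay it finds the GridBehaviours actor, then linearly scans every tile for the one nearest its location.
; It rewrites that tile's struct entry with itself in the unit slot, despite the function being named Get Unit on Tile, then moves to the tile's world location.
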(event `self.ReceiveBeginPlay`
  (`KismetSystemLibrary.Delay` 0.2)
  (bind _returnvalue (`GameplayStatics.GetActorOfClass` "/Game/01_BP/Grid/GridBehaviours.GridBehaviours_C"))
  (set `self.Grid` _returnvalue)
  (`self.Set Grid Index and Snap To Location`))

(fn `Get Unit on Tile`
  (params (`grid Index` :type "Vector2D Structure"))
  (bind _struct_tiles (`/Game/01_BP/Grid/GridBehaviours.struct_Tiles` (`self.Grid`)))
  (bind _struct_tiles_2 (`/Game/01_BP/Grid/GridBehaviours.struct_Tiles` (`self.Grid`)))
  (bind _value (`BlueprintMapLibrary.Map_Find` _struct_tiles (`self.grid Index`)))
  (bind _value_2 (`BlueprintMapLibrary.Map_Find` _struct_tiles_2 (`self.grid Index`)))
  (`BlueprintMapLibrary.Map_Add` _struct_tiles_2 (`self.grid Index`) (make `/Game/01_BP/Structure/Tiles_Struct` (break `/Game/01_BP/Structure/Tiles_Struct` _value_2) null (`.TileCost_25_E8B2FB4843A4F6511FCE96B956F4CC49` (break `/Game/01_BP/Structure/Tiles_Struct` _value_2)) (`.m_TypesOfTile_9_31305E934CC54E66306D4C98AE8F7317` (break `/Game/01_BP/Structure/Tiles_Struct` _value_2)) (`.m_Tiles_WorldLocation_10_52D11E814B5D8A10CE64A1B92294C51C` (break `/Game/01_BP/Structure/Tiles_Struct` _value_2)) (`.m_Tiles_Index_12_B076B1C84440D5EFB37DCB994C2C5E0D` (break `/Game/01_BP/Structure/Tiles_Struct` _value_2)) (`.FinalCost_15_B77FE6EF43A9D0ACCFBB1096C6FFE416` (break `/Game/01_BP/Structure/Tiles_Struct` _value_2)) (`.CostFromStart_23_C992136B48163377F33CDA81F5636A42` (break `/Game/01_BP/Structure/Tiles_Struct` _value_2)) (`.EstimatedCostToTarget_24_C47FE59D4B8F3F2A8DE547A5636A679B` (break `/Game/01_BP/Structure/Tiles_Struct` _value_2)) (`.PreviousTiles_30_1BEEBC784B5F6804CEC6EFA0F6234E00` (break `/Game/01_BP/Structure/Tiles_Struct` _value_2))))
  (set `self.grid Index` `grid Index`)
  (`BlueprintMapLibrary.Map_Add` _struct_tiles (`self.grid Index`) (make `/Game/01_BP/Structure/Tiles_Struct` (break `/Game/01_BP/Structure/Tiles_Struct` _value) self (`.TileCost_25_E8B2FB4843A4F6511FCE96B956F4CC49` (break `/Game/01_BP/Structure/Tiles_Struct` _value)) (`.m_TypesOfTile_9_31305E934CC54E66306D4C98AE8F7317` (break `/Game/01_BP/Structure/Tiles_Struct` _value)) (`.m_Tiles_WorldLocation_10_52D11E814B5D8A10CE64A1B92294C51C` (break `/Game/01_BP/Structure/Tiles_Struct` _value)) (`.m_Tiles_Index_12_B076B1C84440D5EFB37DCB994C2C5E0D` (break `/Game/01_BP/Structure/Tiles_Struct` _value)) (`.FinalCost_15_B77FE6EF43A9D0ACCFBB1096C6FFE416` (break `/Game/01_BP/Structure/Tiles_Struct` _value)) (`.CostFromStart_23_C992136B48163377F33CDA81F5636A42` (break `/Game/01_BP/Structure/Tiles_Struct` _value)) (`.EstimatedCostToTarget_24_C47FE59D4B8F3F2A8DE547A5636A679B` (break `/Game/01_BP/Structure/Tiles_Struct` _value)) (`.PreviousTiles_30_1BEEBC784B5F6804CEC6EFA0F6234E00` (break `/Game/01_BP/Structure/Tiles_Struct` _value)))))

(fn `Set Grid Index and Snap To Location`
  (locals (ClosesDistace :type "Float (double-precision)" :default 1000000000.0) (ClosesIndex :type "Vector2D Structure"))
  (bind _grid (`self.Grid`))
  (bind _struct_tiles (`/Game/01_BP/Grid/GridBehaviours.struct_Tiles` _grid))
  (bind _keys (`BlueprintMapLibrary.Map_Keys` _struct_tiles))
  (for _array_element _keys
    (bind _value (`BlueprintMapLibrary.Map_Find` _struct_tiles _array_element))
    (bind _returnvalue (`KismetMathLibrary.VSize` (- (`.m_Tiles_WorldLocation_10_52D11E814B5D8A10CE64A1B92294C51C` (break `/Game/01_BP/Structure/Tiles_Struct` _value)) (`self.K2_GetActorLocation` self))))
    (if (< _returnvalue (`local.ClosesDistace`))
      (set `local.ClosesDistace` _returnvalue)
      (bind _output_get (set `local.ClosesIndex` (`.m_Tiles_Index_12_B076B1C84440D5EFB37DCB994C2C5E0D` (break `/Game/01_BP/Structure/Tiles_Struct` _value))))
      (`KismetSystemLibrary.PrintString` (`KismetStringLibrary.Conv_Vector2dToString` _output_get))))
  (`self.Get Unit On Tile` (`local.ClosesIndex`))
  (`self.K2_SetActorLocation` (`.m_Tiles_WorldLocation_10_52D11E814B5D8A10CE64A1B92294C51C` (break `/Game/01_BP/Structure/Tiles_Struct` (`BlueprintMapLibrary.Map_Find` (`/Game/01_BP/Grid/GridBehaviours.struct_Tiles` _grid) (`local.ClosesIndex`))))))

(fn `UserConstructionScript`)