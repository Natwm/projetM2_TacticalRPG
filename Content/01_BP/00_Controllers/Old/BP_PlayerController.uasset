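; Player controller for click-to-move control of the pawn, with unit selection tracking and an obstacle visibility toggle.
; While SetDestination is held, a Tick gate traces under the cursor and calls SimpleMoveToLocation, ignoring points too close to the pawn.
; R flip-flops showing and hiding all BP_Base_Obstacle actors, and selection events deselect the previous unit.
; The path event, clicked-tile lookup and possess-on-click logic are unfinished or disconnected.
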(event `self.ReceiveBeginPlay`
  ;[1 1 1] Start
  (bind _returnvalue (`GameplayStatics.GetActorOfClass` "/Game/01_BP/Grid/GridBehaviours.GridBehaviours_C"))
  (set `self.Grid Manager` _returnvalue))

(event `self.ReceiveTick`
  (params (DeltaSeconds :type "Float (single-precision)"))
  ;[1 1 1] Click and go there
  (`|ExecutionSequence`
    (:`then_0`
      (`/Engine/EditorBlueprintResources/StandardMacros.Gate` true :!label _label ; While key is pressed...
        (:`Exit`
          (`self.Move to Hit Location` (`.Location` (`GameplayStatics.BreakHitResult` (`self.GetHitResultUnderCursorByChannel` "TraceTypeQuery1")))))))))

(event `InputAction|SetDestination`
  (params (Key :type "Key Structure"))
  ;[1 1 1] Click and go there
  (:`Pressed`
    (goto _label :!via `Open`))
  (:`Released`
    (goto _label :!via `Close`)))

(event `InputAction|SetDestination`
  (params (Key :type "Key Structure"))
  (:`Pressed`
    ;[1 1 1] HighLight Selected Tiles
    (`KismetSystemLibrary.FlushPersistentDebugLines`)))

(event `Key|R`
  (params (Key :type "Key Structure"))
  (:`Pressed`
    (`/Engine/EditorBlueprintResources/StandardMacros.FlipFlop`
      (:`A`
        (bind _outactors (`GameplayStatics.GetAllActorsOfClass` "/Game/01_BP/Obstacles/BP_Base_Obstacle.BP_Base_Obstacle_C"))
        (for _array_element _outactors
          (`self.SetActorHiddenInGame` _array_element false)))
      (:`B`
        (bind _outactors_2 (`GameplayStatics.GetAllActorsOfClass` "/Game/01_BP/Obstacles/BP_Base_Obstacle.BP_Base_Obstacle_C"))
        (for _array_element_2 _outactors_2
          (`self.SetActorHiddenInGame` _array_element_2 true))))))

(event `E_NewUnitSelected`
  (params (Unit :type "/Game/01_BP/00_Controllers/Old/BP_Unit Object Reference"))
  (`/Engine/EditorBlueprintResources/StandardMacros.IsValid` Unit
    (:`Is Valid`
      (`/Game/01_BP/00_Controllers/Old/BP_Unit.E_DeSelected` (`self.SelectedUnit`)))
    (:`Is Not Valid`
      _))
  (set `self.SelectedUnit` Unit))

(event `E_NewPathAvailable`
  (params (Path :type "Array of Vector2D Structure"))
  (`/Engine/EditorBlueprintResources/StandardMacros.IsValid` (`self.SelectedUnit`)))

(fn `Get World Cliked Tile`
  (returns (`Tile Position` :type "Vector Structure"))
  (return (0.0 0.0 0.0)))

(fn `Move to Hit Location`
  (params (InputPin :type "Vector Structure"))
  (if (>= (`KismetMathLibrary.VSize` (- (`self.K2_GetActorLocation` (`self.K2_GetPawn`)) InputPin)) (`self.Min Click Distance`))
    (`AIBlueprintHelperLibrary.SimpleMoveToLocation` self InputPin)))

(fn `UserConstructionScript`)