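; BP_Unit is a clickable grid unit that snaps to the nearest tile on BeginPlay and reports selection clicks to BP_PlayerController.
; It linearly searches the GridBehaviours tile map for the closest world location, stores that index and moves itself there.
; Clicks on either cone or the capsule always notify the controller, firing the selected event only if not already selected.
; Its selected and deselected events are empty stubs.
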(event `self.ReceiveBeginPlay`
  (set `self.PlayerController` (cast `/Game/01_BP/00_Controllers/Old/BP_PlayerController` (`GameplayStatics.GetPlayerController` 0) :!pure true))
  (bind _returnvalue (`GameplayStatics.GetActorOfClass` "/Game/01_BP/Grid/GridBehaviours.GridBehaviours_C"))
  (set `self.Grid` _returnvalue)
  (`self.SetGridIndexAndSnap`))

(event `self.Cone.OnClicked`
  (params (TouchedComponent :type "PrimitiveComponent Object Reference") (ButtonPressed :type "Key Structure"))
  (if (!= (`/Game/01_BP/00_Controllers/Old/BP_PlayerController.SelectedUnit` (`self.PlayerController`)) self) :!label _label
    (`/Game/01_BP/00_Controllers/Old/BP_PlayerController.E_NewUnitSelected` (`self.PlayerController`) self)
    (`self.E_Selected`)
    (else
      (`/Game/01_BP/00_Controllers/Old/BP_PlayerController.E_NewUnitSelected` (`self.PlayerController`) self))))

(event `self.Cone1.OnClicked`
  (params (TouchedComponent :type "PrimitiveComponent Object Reference") (ButtonPressed :type "Key Structure"))
  (goto _label))

(event `self.CapsuleComponent.OnClicked`
  (params (TouchedComponent :type "PrimitiveComponent Object Reference") (ButtonPressed :type "Key Structure"))
  (goto _label))

(event `E_Selected`)

(event `E_DeSelected`)

(fn `SetGridIndexAndSnap`
  (locals (ClosestDistance :type "Float (double-precision)" :default 0.0) (ClosestIndex :type "Vector2D Structure"))
  (set `local.ClosestDistance` 10000000000.0)
  (bind _keys (`BlueprintMapLibrary.Map_Keys` (`/Game/01_BP/Grid/GridBehaviours.struct_Tiles` (`self.Grid`))))
  (for _array_element _keys
    (bind _value (`BlueprintMapLibrary.Map_Find` (`/Game/01_BP/Grid/GridBehaviours.struct_Tiles` (`self.Grid`)) _array_element))
    (bind _returnvalue (`KismetMathLibrary.VSize` (- (`self.K2_GetActorLocation` self) (`.m_Tiles_WorldLocation_10_52D11E814B5D8A10CE64A1B92294C51C` (break `/Game/01_BP/Structure/Tiles_Struct` _value)))))
    (if (< _returnvalue (`local.ClosestDistance`))
      (set `local.ClosestDistance` _returnvalue)
      (set `local.ClosestIndex` (`.m_Tiles_Index_12_B076B1C84440D5EFB37DCB994C2C5E0D` (break `/Game/01_BP/Structure/Tiles_Struct` _value)))))
  (bind _output_get (set `self.Grid Index` (`local.ClosestIndex`)))
  (`self.K2_SetActorLocation` (`.m_Tiles_WorldLocation_10_52D11E814B5D8A10CE64A1B92294C51C` (break `/Game/01_BP/Structure/Tiles_Struct` (`BlueprintMapLibrary.Map_Find` (`/Game/01_BP/Grid/GridBehaviours.struct_Tiles` (`self.Grid`)) _output_get)))))

(fn `UserConstructionScript`)